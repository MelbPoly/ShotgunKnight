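; Lobby game mode for multiplayer: on login it registers each player, pushes server and map info to their LobbyPC, and spawns them as CodyTestPlayer at a random PlayerStart.
; It relays map settings, player lists and character availability to all controllers, and handles character swaps and kicks.
; A readiness flag tracks character selection; launch server-travels to Forest2 for both map IDs.
; Logout cleanup is disconnected, so departing players are never removed.
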(event Custom|swapcharacter
  (params (player%20controller :type Player%20Controller%20Object%20Reference) (characterClass :type Character%20Class%20Reference) (changedStatus :type Boolean))
  (bind _returnvalue (Pawn|GetControlledPawn player%20controller))
  (bind _spawnpoints (Variables|seversetting|Getspawnpoints))
  ;[1 1 1] swaps current charcater with the selected charcater from charcater select screen
  (if (not changedStatus)
    (Utilities|IsValid _returnvalue
      (:Is%20Valid
        (Actor|DestroyActor _returnvalue))
      (:Is%20Not%20Valid
        _))
    (bind _returnvalue_2 (Game|SpawnActorfromClass characterClass (Transformation|GetActorTransform (Utilities|Array|Get(acopy) _spawnpoints (Math|Random|RandomIntegerinRange 0 (- (Utilities|Array|Length _spawnpoints) 1)))) "Undefined" 0 0))
    (Pawn|Possess player%20controller _returnvalue_2)))

(event Custom|respawnplayers
  (params (playercontroller :type Player%20Controller%20Object%20Reference))
  (bind _returnvalue (Pawn|GetControlledPawn playercontroller))
  (bind _spawnpoints (Variables|seversetting|Getspawnpoints))
  ;[1 1 1] spawn the player as base player when arriving to the lobby
  (Utilities|IsValid _returnvalue
    (:Is%20Valid
      (Actor|DestroyActor _returnvalue))
    (:Is%20Not%20Valid
      _))
  (bind _returnvalue_2 (Game|SpawnActorfromClass "/Game/SimpleWeapon/Blueprints/Character/CodyTestPlayer.CodyTestPlayer_C" (Transformation|GetActorTransform (Utilities|Array|Get(acopy) _spawnpoints (Math|Random|RandomIntegerinRange 0 (- (Utilities|Array|Length _spawnpoints) 1)))) "Undefined" 0 0))
  (Pawn|Possess playercontroller _returnvalue_2)
  (CallFunction|Everyoneapdate))

(event Custom|everyoneapdate
  (bind _allplayercontrollers (Variables|seversetting|Getallplayercontrollers))
  ;[1 1 1] all connected players lobby info when called
  (bind _output_get (Variables|seversetting|Setcurrentplayers (Utilities|Array|Length (Variables|seversetting|Getallplayercontrollers))))
  (if (> _output_get 0)
    (Utilities|Array|Clear (Variables|seversetting|Getconnectedplayer))
    (for _array_element _allplayercontrollers
      (bind _aslobby_pc (Utilities|Casting|CastToLobbyPC _array_element))
      (Utilities|Array|Add (Variables|seversetting|Getconnectedplayer) (Variables|/Game/muiltplayer/Blueprints/Lobby/LobbyPC.LobbyPC_C|Getplayersettings _aslobby_pc))
      (Default|Updatenumberofplayers _aslobby_pc (Variables|seversetting|Getcurrentplayers) (Variables|seversetting|Getmaxplayers)))
    (for _array_element_2 _allplayercontrollers
      (bind _aslobby_pc_2 (Utilities|Casting|CastToLobbyPC _array_element_2))
      (Default|Addplayerinfo _aslobby_pc_2 (Variables|seversetting|Getconnectedplayer))
      (Default|UpdateAvalibleCharacters _aslobby_pc_2 (Variables|seversetting|Getavaliblecharacaters))
      (CallFunction|Addtokicklist))
    (bind _array_element_3 (Utilities|Array|ForEachLoopwithBreak (Variables|seversetting|Getconnectedplayer))
      (:LoopBody
        (if (== (.MyPlayerCharacter (Utilities|Struct|BreakPlayerInfo _array_element_3)) "/Game/SimpleWeapon/Blueprints/Character/CodyTestPlayer.CodyTestPlayer_C")
          (Variables|seversetting|SetCanWeStart? false)
          (CallFunction|Cannotstartgame)
          (else
            (Variables|seversetting|SetCanWeStart? true)))))))

(event Custom|launchthegame
  (bind _returnvalue (Game|GetPlayerController 0))
  ;[1 1 1] launch game on map selection
  (switch int (Variables|seversetting|GetGM_MAPID)
    (:0
      (Development|ExecuteConsoleCommand "servertravel /Game/Map/Forest2" _returnvalue))
    (:1
      (Development|ExecuteConsoleCommand "servertravel /Game/Map/Forest2" _returnvalue))))

(event Custom|addtokicklist
  ;[1 1 1] add player to kick list if a game settings is open
  (bind _aslobby_pc (Utilities|Casting|CastToLobbyPC (Game|GetPlayerController 0)))
  (Utilities|IsValid (Variables|/Game/muiltplayer/Blueprints/Lobby/LobbyPC.LobbyPC_C|GetlobbymenuWB _aslobby_pc)
    (:Is%20Valid
      (if (Widget|IsVisible (Variables|/Game/muiltplayer/UI/Lobby/LobbyMenu.LobbyMenu_C|GetGameSettings (Variables|/Game/muiltplayer/Blueprints/Lobby/LobbyPC.LobbyPC_C|GetlobbymenuWB _aslobby_pc)))
        (Default|FillPlayerWindow (Variables|/Game/muiltplayer/UI/Lobby/LobbyMenu.LobbyMenu_C|GetGameSettings (Variables|/Game/muiltplayer/Blueprints/Lobby/LobbyPC.LobbyPC_C|GetlobbymenuWB _aslobby_pc)))))))

(event Custom|cannotstartgame
  ;[1 1 1] all connected players lobby info when called
  (Utilities|Array|ForEachLoopwithBreak (Variables|seversetting|Getconnectedplayer)) ; enters at Break
)

(event Custom|serverupdategamesettings
  (params (mapimage :type Texture%202D%20Object%20Reference) (mapname :type Text) (maptime :type Text) (mapid :type Integer))
  ;[1 1 1] server has made changers / tell each clint to update their lobby info
  (Variables|seversetting|SetGM_mapimage mapimage)
  (Variables|seversetting|SetGM_mapname mapname)
  (Variables|seversetting|SetGM_mapTIME maptime)
  (Variables|seversetting|SetGM_MAPID mapid)
  (for _array_element (Variables|seversetting|Getallplayercontrollers)
    (bind _aslobby_pc (Utilities|Casting|CastToLobbyPC _array_element))
    (Default|Updatelobbysettings _aslobby_pc (Variables|seversetting|GetGM_mapimage) (Variables|seversetting|GetGM_mapname) (Variables|seversetting|GetGM_mapTIME))))

(event Custom|youhavebeenkicked
  (params (playerid :type Integer))
  ;[1 1 1] kicked the selected player
  (Default|Kicked (.AsLobby%20PC (Utilities|Casting|CastToLobbyPC (Utilities|Array|Get(acopy) (Variables|seversetting|Getallplayercontrollers) playerid)))))

(event EventPostLogin
  (params (NewPlayer :type Player%20Controller%20Object%20Reference))
  ;[1 1 1] initial setup pccurs on event post login - handles lobby setup on player controller and spawns player
  (Networking|SwitchHasAuthority
    (:Authority
      (Utilities|Array|Add (Variables|seversetting|Getallplayercontrollers) NewPlayer)
      (bind _outactors (Actor|GetAllActorsOfClass "/Script/Engine.PlayerStart"))
      (Variables|seversetting|Setspawnpoints _outactors)
      (bind _asgameinfoinstance (Utilities|Casting|CastToGameinfoinstance (Game|GetGameInstance)))
      (Variables|seversetting|Setsevername (Variables|/Game/muiltplayer/Blueprints/AllLevels/Gameinfoinstance.Gameinfoinstance_C|GetServerName _asgameinfoinstance))
      (Variables|seversetting|Setmaxplayers (Variables|/Game/muiltplayer/Blueprints/AllLevels/Gameinfoinstance.Gameinfoinstance_C|GetMax%20Players _asgameinfoinstance))
      (bind _aslobby_pc (Utilities|Casting|CastToLobbyPC NewPlayer))
      (Default|Initialsetup _aslobby_pc)
      (Default|Setuplobbymenu _aslobby_pc (Variables|seversetting|Getsevername))
      (Default|Updatelobbysettings _aslobby_pc (Variables|seversetting|GetGM_mapimage) (Variables|seversetting|GetGM_mapname) (Variables|seversetting|GetGM_mapTIME))
      (CallFunction|Respawnplayers NewPlayer))))

(event EventOnLogout
  (params (ExitingController :type Controller%20Object%20Reference))
  (bind _allplayercontrollers (Variables|seversetting|Getallplayercontrollers))
  ;[1 1 1] logout- removes player controller and conneccted player inf/ resets available character
  (bind (_array_element _array_index) (Utilities|Array|ForEachLoopwithBreak _allplayercontrollers :!label _label)
    (:LoopBody
      (if (== _array_element ExitingController)
        (goto _label Break)))
    (:Completed
      (bind _aslobby_pc (Utilities|Casting|CastToLobbyPC (Utilities|Array|Get(acopy) _allplayercontrollers _array_index))))))

(fn ConstructionScript)