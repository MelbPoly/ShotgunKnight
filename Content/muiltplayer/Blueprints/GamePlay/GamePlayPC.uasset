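; Multiplayer gameplay player controller that hands saved player info to the server and handles in-game text chat.
; On BeginPlay the local controller clears widgets, loads the save and passes the settings on, so GamePlayGM respawns the chosen character and the chat widget is created.
; Incoming messages are relayed with the sender's name through the game mode's controller list to update each chat window.
; The T key toggles the mouse cursor.
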(event Custom|passcharcaterinfotoserver
  (params (playersettinginfo :type Player%20Info%20Structure))
  ;[1 1 1] passes character info/ respawns player will character/ calls setup chat window
  (Variables|Default|Setplayersettings playersettinginfo)
  (bind _asgame_play_gm (Utilities|Casting|CastToGamePlayGM (Game|GetGameMode)))
  (Default|Respawnplayer _asgame_play_gm self (.MyPlayerCharacter (Utilities|Struct|BreakPlayerInfo (Variables|Default|Getplayersettings))))
  (CallFunction|SetupChatWindow))

(event Custom|updatechat
  (params (sender%20name :type Text) (sender%20text :type Text))
  ;[1 1 1] update the clinet chat window
  (Default|Updatechatwindow (Variables|/Game/muiltplayer/UI/AllLevels/GameplayChat.GameplayChat_C|Getgameplaychat (Variables|Default|Getgame%20play%20chat)) sender%20name sender%20text))

(event Custom|setup%20chat%20window
  ;[1 1 1] add chat to window
  (bind _returnvalue (UserInterface|CreateWidget "/Game/muiltplayer/UI/AllLevels/GameplayChat.GameplayChat_C"))
  (bind _output_get (Variables|Default|Setgame%20play%20chat _returnvalue))
  (UserInterface|Viewport|AddtoViewport _output_get 0))

(event Custom|get%20chat%20meassge
  (params (texttosend :type Text))
  ;[1 1 1] process and hands incoming chat
  (Variables|Default|Setsender%20text texttosend)
  (Variables|Default|Setsender%20name (.MyPlayerName (Utilities|Struct|BreakPlayerInfo (Variables|Default|Getplayersettings))))
  (bind _asgame_play_gm (Utilities|Casting|CastToGamePlayGM (Game|GetGameMode)))
  (for _array_element (Variables|/Game/muiltplayer/Blueprints/GamePlay/GamePlayGM.GamePlayGM_C|Getallplayerconrollers _asgame_play_gm)
    (bind _asgame_play_pc (Utilities|Casting|CastToGamePlayPC _array_element))
    (CallFunction|Updatechat _asgame_play_pc (Variables|Default|Getsender%20name) (Variables|Default|Getsender%20text))))

(event EventBeginPlay
  ;[1 1 1] loads player info and pass to serverside player conrtoller
  (if (Pawn|IsLocalController)
    (Viewport|RemoveAllWidgets)
    (CallFunction|LOADGAME)
    (CallFunction|Passcharcaterinfotoserver (Variables|Default|Getplayersettings))))

(event Input|KeyboardEvents|T
  (params (Key :type Key%20Structure :default "AnyKey"))
  ;[1 1 1] t to type
  (:Pressed
    (Utilities|FlowControl|FlipFlop
      (:A
        (Variables|Default|SetbShowMouseCursor true))
      (:B
        (Variables|Default|SetbShowMouseCursor false)))))

(fn ConstructionScript)

(fn LOADGAME
  (bind _returnvalue (SaveGame|LoadGamefromSlot (Variables|Default|Getplayer%20setting%20save)))
  (bind _asplayer_save_game (Utilities|Casting|CastToPlayerSaveGame _returnvalue))
  (Variables|Default|Setplayersettings (Variables|/Game/muiltplayer/Blueprints/AllLevels/PlayerSaveGame.PlayerSaveGame_C|GetS_PlayerInfo _asplayer_save_game)))